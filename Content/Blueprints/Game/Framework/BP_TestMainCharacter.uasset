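; Test player character with camera-relative movement, look controls, weapon attacks and death handling.
; A state enum gates movement and attacks to Locomotion, and collected weapons attach to a mesh socket.
; Attacks play a montage and bind check start/end events that forward to the weapon.
; Damage feeds a stat component, whose zero-HP event triggers the death montage, disables collision and resets tags.
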(event `self.ReceiveBeginPlay`
  (add `/Game/Blueprints/Game/Component/BPAC_CharacterStat.OnHpZero` (`self.BPAC_CharacterStat`) (delegate `OnPlayerDied`)))

(event `OnPlayerDied`
  (set `self.CharacterState` "NewEnumerator2")
  (`self.PlayAnimMontage` "/Game/Blueprints/Game/Animation/AM_Dead.AM_Dead")
  (`self.SetActorEnableCollision` false)
  (set `self.Tags` (`|MakeArray` "None" :!type "Name")))

(event `EnhancedInput|/Game/Blueprints/Input/IA_Move`
  (params (ActionValue :type "Vector2D Structure") (ElapsedSeconds :type "Float (double-precision)") (TriggeredSeconds :type "Float (double-precision)") (InputAction :type "InputAction Object Reference" :default "/Game/Blueprints/Input/IA_Move.IA_Move"))
  (bind (_returnvalue_roll _returnvalue_pitch _returnvalue_yaw) (`KismetMathLibrary.BreakRotator` (`self.GetControlRotation`)))
  ;[0.07344 0.15 0.06471 0.5] Movement
  (:`Triggered`
    (switch `/Game/Blueprints/Game/Framework/E_CharacterState` (`self.CharacterState`)
      (:`NewEnumerator0`
        (`self.AddMovementInput` (+ (* (`KismetMathLibrary.GetRightVector` (`KismetMathLibrary.MakeRotator` 0.0 0.0 _returnvalue_yaw)) ActionValue_X) (* (`KismetMathLibrary.GetForwardVector` (`KismetMathLibrary.MakeRotator` 0.0 0.0 _returnvalue_yaw)) ActionValue_Y)))))))

(event `EnhancedInput|/Game/Blueprints/Input/IA_Look`
  (params (ActionValue :type "Vector2D Structure") (ElapsedSeconds :type "Float (double-precision)") (TriggeredSeconds :type "Float (double-precision)") (InputAction :type "InputAction Object Reference" :default "/Game/Blueprints/Input/IA_Look.IA_Look"))
  ;[0.15 0.1364 0.07125 0.5] Camera Rotation
  (:`Triggered`
    (`|ExecutionSequence`
      (:`then_0`
        (`self.AddControllerYawInput` ActionValue_X))
      (:`then_1`
        (`self.AddControllerPitchInput` (* ActionValue_Y -1.0))))))

(event `OnWeaponCollected`
  (params (Weapon :type "/Game/Blueprints/Game/Actor/BP_Weapon Object Reference"))
  ;[0.1011 0.08161 0.15 0.5] 무기 획득 처리
  (bind _output_get (set `self.Weapon` Weapon))
  (`self.K2_AttachToComponent` _output_get (`self.Mesh`) "WeaponPosition" "SnapToTarget" "SnapToTarget" "SnapToTarget" true))

(event `EnhancedInput|/Game/Blueprints/Input/IA_Attack`
  (params (ActionValue :type Boolean) (ElapsedSeconds :type "Float (double-precision)") (TriggeredSeconds :type "Float (double-precision)") (InputAction :type "InputAction Object Reference" :default "/Game/Blueprints/Input/IA_Attack.IA_Attack"))
  ;[0.15 0.04445 0.04674 0.5] Attack
  (:`Started`
    (`self.OnAttack`)))

(event `OnAttack`
  ;[0.15 0.05268 0.04788 0.5] Attack [Start & End]
  (`self.Weapon`
    (:`then`
      (switch `/Game/Blueprints/Game/Framework/E_CharacterState` (`self.CharacterState`)
        (:`NewEnumerator0`
          (set `self.CharacterState` "NewEnumerator1")
          (`AnimInstance.Montage_Play` (`SkeletalMeshComponent.GetAnimInstance` (`self.Mesh`)) "/Game/Blueprints/Game/Animation/AM_Attack.AM_Attack" 1.0 "MontageLength" 0.0 true)
          (add `self.AttackCheckStart` (delegate `OnAttackCheckStart`))
          (add `self.AttackCheckEnd` (delegate `OnAttackCheckEnd`)))))
    (:`else`)))

(event `OnAttackCheckStart`
  ;[0.15 0.05268 0.04788 0.5] Attack [Start & End]
  (`/Game/Blueprints/Game/Actor/BP_Weapon.OnAttackCheckStart` (`self.Weapon`)))

(event `OnAttackCheckEnd`
  (`/Game/Blueprints/Game/Actor/BP_Weapon.OnAttackCheckEnd` (`self.Weapon`)))

(event `OnAttackEnd`
  ;[0.15 0.05268 0.04788 0.5] Attack [Start & End]
  (set `self.CharacterState` "NewEnumerator0"))

(event `self.ReceiveAnyDamage`
  (params (Damage :type "Float (single-precision)") (DamageType :type "DamageType Object Reference") (InstigatedBy :type "Controller Object Reference") (DamageCauser :type "Actor Object Reference"))
  (`/Game/Blueprints/Game/Component/BPAC_CharacterStat.ReceiveDamage` (`self.BPAC_CharacterStat`) Damage))

(fn `UserConstructionScript`)