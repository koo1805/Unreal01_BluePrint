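; BP_EnemyBear is a bear enemy that takes damage, flashes when hit and dies.
; Any damage is forwarded to the BPACMonsterStat component and restarts a timeline that drives the DamageFactor parameter on a dynamic material instance of the stone bear material.
; When that component signals zero HP, the bear disables collision, plays its death montage and destroys itself after a short delay.
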(event `self.ReceiveBeginPlay`
  (bind _returnvalue (`PrimitiveComponent.CreateDynamicMaterialInstance` (`self.Mesh`) 0 "/Game/InfinityBladeAdversaries/Enemy/Enemy_Bear/Materials/M_Bear_Stone_Inst.M_Bear_Stone_Inst" "None"))
  (set `self.MI_Damage` _returnvalue)
  (add `/Game/Blueprints/Game/Component/BPAC_MonsterStat.OnHpZero` (`self.BPAC_MonsterStat`) (delegate `MonsterDied`)))

(event `MonsterDied`
  ;[0.06068 0.08909 0.15 0.5] Hp To Zero
  (`self.SetActorEnableCollision` false)
  (`AnimInstance.Montage_Play` (`SkeletalMeshComponent.GetAnimInstance` (`self.Mesh`)) "/Game/Blueprints/Game/Enemy/AnimMontage_BearDeath.AnimMontage_BearDeath" 1.0 "MontageLength" 0.0 true)
  (`KismetSystemLibrary.Delay` 2.0)
  (`self.K2_DestroyActor`))

(event `self.ReceiveAnyDamage`
  (params (Damage :type "Float (single-precision)") (DamageType :type "DamageType Object Reference") (InstigatedBy :type "Controller Object Reference") (DamageCauser :type "Actor Object Reference"))
  ;[0.06429 0.15 0.04888 0.5] Damage
  (`self.PlayDamageEffect`)
  (`/Game/Blueprints/Game/Component/BPAC_MonsterStat.RecieveDamage` (`self.BPAC_MonsterStat`) Damage))

(event `PlayDamageEffect`
  ;[0.15 0.06646 0.05641 0.5] Damage Effect
  (bind (_direction _alpha) (`Timeline|DamageEffect` :!via `PlayFromStart`)
    (:`Update`
      (bind _mi_damage (`self.MI_Damage`)
        (:`then`
          (`MaterialInstanceDynamic.SetScalarParameterValue` _mi_damage "DamageFactor" _alpha))
        (:`else`)))))

(fn `UserConstructionScript`)