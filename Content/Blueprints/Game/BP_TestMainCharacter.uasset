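; BP_TestMainCharacter is a test player character that handles basic movement and camera look through Enhanced Input actions.
; IA_Move builds forward and right vectors from control-rotation yaw alone, scales them by the input axes and feeds the sum to AddMovementInput.
; IA_Look drives controller yaw from X and pitch from negated Y.
; The construction script is empty.
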(event `EnhancedInput|/Game/Blueprints/Input/IA_Move`
  (params (ActionValue :type "Vector2D Structure") (ElapsedSeconds :type "Float (double-precision)") (TriggeredSeconds :type "Float (double-precision)") (InputAction :type "InputAction Object Reference" :default "/Game/Blueprints/Input/IA_Move.IA_Move"))
  (bind (_returnvalue_roll _returnvalue_pitch _returnvalue_yaw) (`KismetMathLibrary.BreakRotator` (`self.GetControlRotation`)))
  ;[0.07344 0.15 0.06471 0.5] Movement
  (:`Triggered`
    (`self.AddMovementInput` (+ (* (`KismetMathLibrary.GetRightVector` (`KismetMathLibrary.MakeRotator` 0.0 0.0 _returnvalue_yaw)) ActionValue_X) (* (`KismetMathLibrary.GetForwardVector` (`KismetMathLibrary.MakeRotator` 0.0 0.0 _returnvalue_yaw)) ActionValue_Y)))))

(event `EnhancedInput|/Game/Blueprints/Input/IA_Look`
  (params (ActionValue :type "Vector2D Structure") (ElapsedSeconds :type "Float (double-precision)") (TriggeredSeconds :type "Float (double-precision)") (InputAction :type "InputAction Object Reference" :default "/Game/Blueprints/Input/IA_Look.IA_Look"))
  ;[0.15 0.1364 0.07125 0.5] Camera Rotation
  (:`Triggered`
    (`|ExecutionSequence`
      (:`then_0`
        (`self.AddControllerYawInput` ActionValue_X))
      (:`then_1`
        (`self.AddControllerPitchInput` (* ActionValue_Y -1.0))))))

(fn `UserConstructionScript`)