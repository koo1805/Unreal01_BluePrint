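; Level-streaming trigger actor that alternates between loading and unloading test sublevels each time a Player-tagged actor begins overlapping it.
; The IsOver flag starts true, so the first overlap does a blocking, visible load of TestMap02_Sub02 and clears the flag.
; The next overlap unloads TestMap02_Sub01, rather than the loaded Sub02, and sets the flag again.
; An unconnected branch comparing and unloading SelectedLevel never runs.
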(event `self.ReceiveBeginPlay`
  (set `self.SelectedLevel` "/Game/Maps/TestMap02_Sub01.TestMap02_Sub01")
  (set `self.IsOver` true))

(event `self.ReceiveActorBeginOverlap`
  (params (OtherActor :type "Actor Object Reference"))
  (if (`self.ActorHasTag` OtherActor "Player")
    (if (`self.IsOver`)
      (bind _output_get (set `self.SelectedLevel` "/Game/Maps/TestMap02_Sub02.TestMap02_Sub02"))
      (`GameplayStatics.LoadStreamLevelBySoftObjectPtr` _output_get true true)
      (set `self.IsOver` false)
      (else
        (`GameplayStatics.UnloadStreamLevelBySoftObjectPtr` "/Game/Maps/TestMap02_Sub01.TestMap02_Sub01")
        (set `self.IsOver` true)))))

(fn `UserConstructionScript`)