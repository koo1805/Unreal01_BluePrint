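; BP_Cow is a toy cow gimmick that launches the player upward on contact.
; A dynamic material instance, created on BeginPlay, switches BodyColor to a collide color while anything overlaps its Box and restores the origin color when an overlap ends.
; Characters tagged Player receive a vertical velocity-change impulse scaled by PushPower.
; Any damage spawns a ground-impact particle effect at the cow's location.
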(event `self.ReceiveBeginPlay`
  (bind _returnvalue (`PrimitiveComponent.CreateDynamicMaterialInstance` (`self.SM_Cow`) 0 "/Game/Wanted_Dev/ToyCow/M_ToyCow.M_ToyCow" "None"))
  (bind _output_get (set `self.MI_Cow` _returnvalue))
  (`MaterialInstanceDynamic.SetVectorParameterValue` _output_get "BodyColor" (`self.OriginColor`)))

(event `self.Box.OnComponentBeginOverlap`
  (params (OverlappedComponent :type "PrimitiveComponent Object Reference") (OtherActor :type "Actor Object Reference") (OtherComp :type "PrimitiveComponent Object Reference") (OtherBodyIndex :type Integer) (bFromSweep :type Boolean) (SweepResult :type "HitResult Structure (by ref)"))
  (`MaterialInstanceDynamic.SetVectorParameterValue` (`self.MI_Cow`) "BodyColor" (`self.CollideColor`))
  (if (`self.ActorHasTag` OtherActor "Player")
    (bind _ascharacter (cast `Character` OtherActor))
    (`CharacterMovementComponent.AddImpulse` (`Character.CharacterMovement` _ascharacter) (* (`KismetMathLibrary.MakeVector` 0.0 0.0 1.0) (`self.PushPower`)) true)))

(event `self.Box.OnComponentEndOverlap`
  (params (OverlappedComponent :type "PrimitiveComponent Object Reference") (OtherActor :type "Actor Object Reference") (OtherComp :type "PrimitiveComponent Object Reference") (OtherBodyIndex :type Integer))
  (`MaterialInstanceDynamic.SetVectorParameterValue` (`self.MI_Cow`) "BodyColor" (`self.OriginColor`)))

(event `self.ReceiveAnyDamage`
  (params (Damage :type "Float (single-precision)") (DamageType :type "DamageType Object Reference") (InstigatedBy :type "Controller Object Reference") (DamageCauser :type "Actor Object Reference"))
  (`GameplayStatics.SpawnEmitterAtLocation` "/Game/Particles/P_GroundImpact.P_GroundImpact" (`self.K2_GetActorLocation`)))

(fn `UserConstructionScript`)