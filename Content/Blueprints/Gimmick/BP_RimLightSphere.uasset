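; BP_RimLightSphere is a gimmick actor that knocks the player away on contact and plays a material effect on its sphere.
; BeginPlay creates a dynamic instance of M_Sphere on the Sphere component.
; When a Player-tagged Character overlaps, it receives a velocity-change impulse away from the actor's center, scaled by PushPower and the unnormalized offset.
; The same overlap restarts the TurnOn timeline, which drives the material's Alpha parameter.
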(event `self.ReceiveBeginPlay`
  (bind _returnvalue (`PrimitiveComponent.CreateDynamicMaterialInstance` (`self.Sphere`) 0 "/Game/Materials/Rimlight/M_Sphere.M_Sphere" "Alpha"))
  (set `self.MI_Sphere` _returnvalue))

(event `self.ReceiveActorBeginOverlap`
  (params (OtherActor :type "Actor Object Reference"))
  (if (`self.ActorHasTag` OtherActor "Player")
    (bind _ascharacter (cast `Character` OtherActor))
    (`CharacterMovementComponent.AddImpulse` (`Character.CharacterMovement` _ascharacter) (* (- (`self.K2_GetActorLocation` self) (`self.K2_GetActorLocation` _ascharacter)) (* -1.0 (`self.PushPower`))) true)
    (bind (_direction _alpha) (`Timeline|TurnOn` :!via `PlayFromStart`)
      (:`Update`
        (`MaterialInstanceDynamic.SetScalarParameterValue` (`self.MI_Sphere`) "Alpha" _alpha)))))

(fn `UserConstructionScript`)